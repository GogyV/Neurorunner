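; Collectible pickup actor that tracks collection progress and triggers the win volume's move once enough are gathered.
; The inherited Pickup event increments CollectibleCount on player 0's state, while sphere overlap separately increments the character's Pickups counter.
; At six or more, the overlap shows an all-pickups notification widget and a timeline lerps BP_WinVolume between hard-coded locations.
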(event `self.Pickup`
  (params (`Player Pawn` :type "Pawn Object Reference"))
  (`parent.Pickup` `Player Pawn`)
  (bind _asbp_third_person_player_state (cast `/Game/_Game/Blueprints/BP_ThirdPersonPlayerState` (`GameplayStatics.GetPlayerState` 0)))
  (`/Engine/EditorBlueprintResources/StandardMacros.IncrementInt` (`/Game/_Game/Blueprints/BP_ThirdPersonPlayerState.CollectibleCount` _asbp_third_person_player_state)))

(event `self.SphereCollision.OnComponentBeginOverlap`
  (params (OverlappedComponent :type "PrimitiveComponent Object Reference") (OtherActor :type "Actor Object Reference") (OtherComp :type "PrimitiveComponent Object Reference") (OtherBodyIndex :type Integer) (bFromSweep :type Boolean) (SweepResult :type "HitResult Structure (by ref)"))
  (bind _asbp_third_person_character (cast `/Game/ThirdPerson/Blueprints/BP_ThirdPersonCharacter` OtherActor))
  (bind _pickups (`/Game/ThirdPerson/Blueprints/BP_ThirdPersonCharacter.Pickups` _asbp_third_person_character))
  (set `/Game/ThirdPerson/Blueprints/BP_ThirdPersonCharacter.Pickups` (+ _pickups 1) _asbp_third_person_character)
  (if (>= _pickups 6)
    (bind _returnvalue (`|CreateWidget` "/Game/_Game/UI/WBP_AllPickupNotification.WBP_AllPickupNotification_C"))
    (`UserWidget.AddToViewport` _returnvalue 0)
    (bind _returnvalue_2 (`GameplayStatics.GetActorOfClass` "/Game/_Game/Blueprints/Actors/BP_WinVolume.BP_WinVolume_C"))
    (bind (_direction _newtrack_0) (`Timeline|Timeline` :!via `PlayFromStart`)
      (:`Update`
        (`SceneComponent.K2_SetRelativeLocation` (`Actor.RootComponent` _returnvalue_2) (`KismetMathLibrary.VLerp` (-14830.0 -168.925224 441.849921) (0.0 0.0 500.0) _newtrack_0) false false)))))

(fn `UserConstructionScript`
  (`parent.UserConstructionScript`))