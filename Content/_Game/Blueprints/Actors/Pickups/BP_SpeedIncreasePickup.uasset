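; Speed boost pickup that temporarily raises the walk speed of the pawn that collects it.
; Its Pickup event finds the pawn's CharacterMovementComponent and, if valid, adds SpeedIncreaseAmount to MaxWalkSpeed.
; After a short fixed Delay it subtracts a separate SpeedDecreaseAmount, so the original speed returns only when both amounts match.
; The construction script only calls its parent.
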(event `self.Pickup`
  (params (`Player Pawn` :type "Pawn Object Reference"))
  (bind _returnvalue (`self.GetComponentByClass` `Player Pawn` "/Script/Engine.CharacterMovementComponent"))
  (`/Engine/EditorBlueprintResources/StandardMacros.IsValid` _returnvalue
    (:`Is Valid`
      (set `CharacterMovementComponent.MaxWalkSpeed` (+ (`CharacterMovementComponent.MaxWalkSpeed` _returnvalue) (`self.SpeedIncreaseAmount`)) _returnvalue)
      (`KismetSystemLibrary.Delay` 2.0)
      (set `CharacterMovementComponent.MaxWalkSpeed` (- (`CharacterMovementComponent.MaxWalkSpeed` _returnvalue) (`self.SpeedDecreaseAmount`)) _returnvalue))))

(fn `UserConstructionScript`
  (`parent.UserConstructionScript`))