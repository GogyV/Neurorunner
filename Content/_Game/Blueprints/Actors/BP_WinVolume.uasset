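; BP_WinVolume is a trigger actor that ends play with a win sequence when the third-person character enters its box.
; On overlap it replaces all widgets with WBP_Win, disables player input, and spawns a teleport effect and win sound at the player's location.
; It then destroys itself, starts a held camera fade-out, and plays win music in 2D.
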(event `self.ReceiveBeginPlay`)

(event `self.Box.OnComponentBeginOverlap`
  (params (OverlappedComponent :type "PrimitiveComponent Object Reference") (OtherActor :type "Actor Object Reference") (OtherComp :type "PrimitiveComponent Object Reference") (OtherBodyIndex :type Integer) (bFromSweep :type Boolean) (SweepResult :type "HitResult Structure (by ref)"))
  (cast `/Game/ThirdPerson/Blueprints/BP_ThirdPersonCharacter` OtherActor)
  (`WidgetLayoutLibrary.RemoveAllWidgets`)
  (bind _returnvalue (`|CreateWidget` "/Game/_Game/UI/WBP_Win.WBP_Win_C"))
  (`UserWidget.AddToViewport` _returnvalue 0)
  (`self.DisableInput` (`GameplayStatics.GetPlayerPawn` 0) null)
  (`NiagaraFunctionLibrary.SpawnSystemAtLocation` "/Game/_Game/Particles/PS_Teleport.PS_Teleport" (`self.K2_GetActorLocation` (`GameplayStatics.GetPlayerPawn` 0)))
  (`GameplayStatics.SpawnSoundAtLocation` "/Game/_Game/Audio/Win_Cue.Win_Cue" (`self.K2_GetActorLocation` (`GameplayStatics.GetPlayerPawn` 0)) (struct) 1.0 1.0 0.0 null null)
  (`self.K2_DestroyActor`)
  (`PlayerCameraManager.StartCameraFade` :`self` (`GameplayStatics.GetPlayerCameraManager` 0) :`ToAlpha` 1.0 :`Duration` 3.0 :`bHoldWhenFinished` true)
  (`GameplayStatics.SpawnSound2D` "/Game/_Game/Audio/WinMusic_Cue.WinMusic_Cue" 0.3 1.0 0.0 null))

(fn `UserConstructionScript`)