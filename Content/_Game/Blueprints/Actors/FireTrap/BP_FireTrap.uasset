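; Fire trap actor that warms up when touched, then becomes lethal for a timed period before returning to idle.
; An enter/exit state machine (Idle, Warming, Hot, Disabled) swaps particles and audio, with timers advancing Warming and Hot.
; The damage volume is live only in Hot; an overlapping Character is destroyed with burst effects, lose widget and camera fade.
; The first BP_DisableActor found in the level can switch it to Disabled.
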(event `self.ReceiveBeginPlay`
  (`PrimitiveComponent.SetCollisionEnabled` (`self.DamageVolume`) "NoCollision")
  (`self.ChangeState` "NewEnumerator0")
  (bind _returnvalue (`GameplayStatics.GetActorOfClass` "/Game/_Game/Blueprints/Actors/Pickups/BP_DisableActor.BP_DisableActor_C"))
  (add `/Game/_Game/Blueprints/Actors/Pickups/BP_DisableActor.DisableTrap` _returnvalue (`|CreateDelegate` :!event `DisableTrap`)))

(event `self.ReceiveTick`
  (params (DeltaSeconds :type "Float (single-precision)"))
  (switch `/Game/_Game/Blueprints/Actors/FireTrap/E_FireTrapState` (`self.CurrentState`)))

(event `self.ActivateVolume.OnComponentBeginOverlap`
  (params (OverlappedComponent :type "PrimitiveComponent Object Reference") (OtherActor :type "Actor Object Reference") (OtherComp :type "PrimitiveComponent Object Reference") (OtherBodyIndex :type Integer) (bFromSweep :type Boolean) (SweepResult :type "HitResult Structure (by ref)"))
  (`self.OnTrapTouched`))

(event `self.DamageVolume.OnComponentBeginOverlap`
  (params (OverlappedComponent :type "PrimitiveComponent Object Reference") (OtherActor :type "Actor Object Reference") (OtherComp :type "PrimitiveComponent Object Reference") (OtherBodyIndex :type Integer) (bFromSweep :type Boolean) (SweepResult :type "HitResult Structure (by ref)"))
  (bind _ascharacter (cast `Character` OtherActor))
  (bind _returnvalue (`|CreateWidget` "/Game/_Game/UI/WBP_Lose.WBP_Lose_C"))
  (`UserWidget.AddToViewport` _returnvalue 0)
  (`NiagaraFunctionLibrary.SpawnSystemAtLocation` "/Game/_Game/Particles/PS_KillBurst.PS_KillBurst" (`self.K2_GetActorLocation` (`GameplayStatics.GetPlayerPawn` 0)))
  (`GameplayStatics.SpawnSoundAtLocation` "/Game/_Game/Audio/DeathBurst_Cue.DeathBurst_Cue" (`self.K2_GetActorLocation` (`GameplayStatics.GetPlayerPawn` 0)) (struct) 1.0 1.0 0.0 null null)
  (`self.K2_DestroyActor` _ascharacter)
  (`PlayerCameraManager.StartCameraFade` :`self` (`GameplayStatics.GetPlayerCameraManager` 0) :`ToAlpha` 1.0 :`Duration` 3.0 :`bShouldFadeAudio` true :`bHoldWhenFinished` true))

(fn `ActivateTrap`
  (`self.ChangeState` "NewEnumerator1"))

(fn `ChangeState`
  (params (NewState :type "/Game/_Game/Blueprints/Actors/FireTrap/E_FireTrapState Enum" :default "NewEnumerator0"))
  (if (`self.IsInitialState`)
    (set `self.IsInitialState` false)
    (set `self.CurrentState` NewState :!label _label)
    (switch `/Game/_Game/Blueprints/Actors/FireTrap/E_FireTrapState` (`self.CurrentState`)
      (:`NewEnumerator0`
        (`self.EnterIdleState`))
      (:`NewEnumerator1`
        (`self.EnterWarmingState`))
      (:`NewEnumerator2`
        (`self.EnterHotState`))
      (:`NewEnumerator3`
        (`self.EnterDisableState`)))
    (elif (not (`|EnumEquality` NewState (`self.CurrentState`)))
      (switch `/Game/_Game/Blueprints/Actors/FireTrap/E_FireTrapState` (`self.CurrentState`)
        (:`NewEnumerator0`
          (`self.ExitIdleState`)
          (goto _label))
        (:`NewEnumerator1`
          (`self.ExitWarmingState`)
          (goto _label))
        (:`NewEnumerator2`
          (`self.ExitHotState`)
          (goto _label))
        (:`NewEnumerator3`
          (`self.ExitDisableState`)
          (goto _label))))))

(fn `DisableTrap`
  (`self.ChangeState` "NewEnumerator3"))

(fn `EnterDisableState`
  (bind _trapparticles (`self.TrapParticles`))
  (`PrimitiveComponent.SetCollisionEnabled` (`self.DamageVolume`) "NoCollision")
  (`NiagaraComponent.SetAsset` _trapparticles (`self.DisableParticles`) true)
  (`ActorComponent.Activate` _trapparticles false)
  (`GameplayStatics.PlaySoundAtLocation` (`self.DisableSound`) (`self.K2_GetActorLocation`) (struct) 1.0 1.0 0.0 null null null null))

(fn `EnterHotState`
  (bind _trapparticles (`self.TrapParticles`))
  (bind _trapaudio (`self.TrapAudio`))
  (`PrimitiveComponent.SetCollisionEnabled` (`self.DamageVolume`) "QueryAndPhysics")
  (`NiagaraComponent.SetAsset` _trapparticles (`self.HotParticles`) true)
  (`ActorComponent.Activate` _trapparticles false)
  (`AudioComponent.SetSound` _trapaudio (`self.HotLoopingSound`))
  (`ActorComponent.Activate` _trapaudio false)
  (`GameplayStatics.PlaySoundAtLocation` (`self.HotActivateSound`) (`self.K2_GetActorLocation`) (struct) 1.0 1.0 0.0 null null null null)
  (`KismetSystemLibrary.K2_SetTimer` null "OnHotTimerEnded" (`self.HotDuration`)))

(fn `EnterIdleState`
  (add `self.OnTrapTouched` (`|CreateDelegate` :!event `ActivateTrap`)))

(fn `EnterWarmingState`
  (bind _trapparticles (`self.TrapParticles`))
  (`NiagaraComponent.SetAsset` _trapparticles (`self.WarmingParticles`) true)
  (`ActorComponent.Activate` _trapparticles false)
  (`GameplayStatics.PlaySoundAtLocation` (`self.ActivateWarmingSound`) (`self.K2_GetActorLocation`) (struct) 1.0 1.0 0.0 null null null null)
  (`KismetSystemLibrary.K2_SetTimer` null "OnWarmingTimerEnded" (`self.WarmingDuration`)))

(fn `ExitDisableState`
  (`PrimitiveComponent.SetCollisionEnabled` (`self.DamageVolume`) "NoCollision")
  (`GameplayStatics.PlaySoundAtLocation` (`self.DisableRe-activateSound`) (`self.K2_GetActorLocation`) (struct) 1.0 1.0 0.0 null null null null)
  (`self.ChangeState` "NewEnumerator0"))

(fn `ExitHotState`
  (`PrimitiveComponent.SetCollisionEnabled` (`self.DamageVolume`) "NoCollision")
  (`ActorComponent.Deactivate` (`self.TrapParticles`))
  (`ActorComponent.Deactivate` (`self.TrapAudio`)))

(fn `ExitIdleState`
  (remove `self.OnTrapTouched` (`|CreateDelegate` :!event `ActivateTrap`)))

(fn `ExitWarmingState`
  (`ActorComponent.Deactivate` (`self.TrapParticles`)))

(fn `OnHotTimerEnded`
  (`self.ChangeState` "NewEnumerator0"))

(fn `OnWarmingTimerEnded`
  (`self.ChangeState` "NewEnumerator2"))

(fn `TickDisableState`)

(fn `TickHotState`)

(fn `TickIdleState`)

(fn `TickWarmingState`)

(fn `UserConstructionScript`)