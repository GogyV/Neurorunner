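; BP_TurretProjectile is a turret projectile that kills any Character entering its DamageVolume, triggering a game-over.
; On overlap it adds the WBP_Lose widget, plays a kill burst effect, death sound and camera shake at the player, then destroys the overlapped Character and fades the camera and audio out.
; Feedback targets player 0 regardless of which Character was hit, and the graph contains no movement logic.
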(event `self.DamageVolume.OnComponentBeginOverlap`
  (params (OverlappedComponent :type "PrimitiveComponent Object Reference") (OtherActor :type "Actor Object Reference") (OtherComp :type "PrimitiveComponent Object Reference") (OtherBodyIndex :type Integer) (bFromSweep :type Boolean) (SweepResult :type "HitResult Structure (by ref)"))
  (bind _ascharacter (cast `Character` OtherActor))
  (bind _returnvalue (`|CreateWidget` "/Game/_Game/UI/WBP_Lose.WBP_Lose_C"))
  (`UserWidget.AddToViewport` _returnvalue 0)
  (`NiagaraFunctionLibrary.SpawnSystemAtLocation` "/Game/_Game/Particles/PS_KillBurst.PS_KillBurst" (`self.K2_GetActorLocation` (`GameplayStatics.GetPlayerPawn` 0)))
  (`LegacyCameraShake.StartLegacyCameraShake` (`GameplayStatics.GetPlayerCameraManager` 0) "/Game/FirstPerson/Blueprints/BP_CameraShake.BP_CameraShake_C" 1.0 "World")
  (`GameplayStatics.SpawnSoundAtLocation` "/Game/_Game/Audio/DeathBurst_Cue.DeathBurst_Cue" (`self.K2_GetActorLocation` (`GameplayStatics.GetPlayerPawn` 0)) (struct) 1.0 1.0 0.0 null null)
  (`self.K2_DestroyActor` _ascharacter)
  (`PlayerCameraManager.StartCameraFade` :`self` (`GameplayStatics.GetPlayerCameraManager` 0) :`ToAlpha` 1.0 :`Duration` 3.0 :`bShouldFadeAudio` true :`bHoldWhenFinished` true))

(fn `UserConstructionScript`)