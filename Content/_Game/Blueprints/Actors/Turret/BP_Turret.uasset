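; BP_Turret is a turret actor that fires at the player character when its PawnSensing component sees one.
; On sighting a BP_ThirdPersonCharacter it turns the whole actor, via TurretTop's owner, toward that pawn.
; After a short Delay, which also throttles repeat sightings, it spawns a BP_TurretProjectile at the Arrow's transform.
; Each shot also spawns a detection-burst effect and a shoot sound, the latter placed at world origin.
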(event `self.PawnSensing.OnSeePawn`
  (params (Pawn :type "Pawn Object Reference"))
  (cast `/Game/ThirdPerson/Blueprints/BP_ThirdPersonCharacter` Pawn)
  (`self.K2_SetActorRotation` (`ActorComponent.GetOwner` (`self.TurretTop`)) (`KismetMathLibrary.FindLookAtRotation` (`self.K2_GetActorLocation`) (`self.K2_GetActorLocation` Pawn)) false)
  (`KismetSystemLibrary.Delay` 0.7)
  (`|SpawnActorFromClass` "/Game/_Game/Blueprints/Actors/Turret/BP_TurretProjectile.BP_TurretProjectile_C" (`SceneComponent.K2_GetComponentToWorld` (`self.Arrow`)) "Undefined" "MultiplyWithRoot" null null)
  (`GameplayStatics.SpawnSoundAtLocation` (`self.Shoot Sound`) (0.0 0.0 0.0) (struct) 1.0 1.0 0.0 null null)
  (`NiagaraFunctionLibrary.SpawnSystemAtLocation` "/Game/_Game/Particles/PS_DetectionBurst.PS_DetectionBurst"))

(fn `UserConstructionScript`)